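; BP_Character is a player character with mouse look, gaze detection of cubes and click-to-teleport movement.
; Every Tick, GazeCheck runs a debug-drawn 2000-unit Visibility trace from the camera and prints colored messages for red or blue cube hits.
; Left Click reuses that trace result to teleport player pawn 0 to the impact point, unless it nearly equals the hit actor's location (70-unit tolerance).
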(event Custom|GazeCheck
  (bind _camera (Variables|Default|GetCamera))
  (bind _returnvalue (Transformation|GetWorldLocation _camera))
  ;[1 1 1] Gaze check
  (bind (_outhit _returnvalue_2) (Collision|LineTraceByChannel _returnvalue (+ _returnvalue (* (Math|Vector|GetForwardVector _camera) 2000)) "TraceTypeQuery1" false 0 "ForOneFrame"))
  (Utilities|Casting|CastToBP_redCube (.HitActor (Collision|BreakHitResult _outhit))
    (:then
      (Development|PrintString "Red Cube Found" true true "(R=1.000000,G=0.152464,B=0.084826,A=1.000000)"))
    (:CastFailed
      (Utilities|Casting|CastToBP_blueCube (.HitActor (Collision|BreakHitResult _outhit)))
      (Development|PrintString "BLUE Cube Found" true true "(R=0.166062,G=0.230617,B=1.000000,A=1.000000)"))))

(event EventTick
  (params (DeltaSeconds :type Float%20%28single-precision%29))
  (CallFunction|GazeCheck))

(event Input|ActionEvents|InputActionLeftClick
  (params (Key :type Key%20Structure :default "None"))
  (:Pressed
    (if (stale Custom|GazeCheck _returnvalue_2)
      ;[1 1 1] Gaze check
      (if (not (Utilities|Operators|EqualEqual (Transformation|GetActorLocation (.HitActor (Collision|BreakHitResult (stale Custom|GazeCheck _outhit)))) (.Location (Collision|BreakHitResult (stale Custom|GazeCheck _outhit))) 7e+01))
        (Transformation|SetActorLocation (Game|Player|GetPlayerPawn 0) (.Location (Collision|BreakHitResult (stale Custom|GazeCheck _outhit))) false true)))))

(event Input|AxisEvents|InputAxismouseX
  (params (AxisValue :type Float%20%28single-precision%29))
  ;[1 1 1] Input
  (Pawn|Input|AddControllerYawInput AxisValue))

(event Input|AxisEvents|InputAxismouseY
  (params (AxisValue :type Float%20%28single-precision%29))
  ;[1 1 1] Input
  (Pawn|Input|AddControllerPitchInput AxisValue))

(fn ConstructionScript)